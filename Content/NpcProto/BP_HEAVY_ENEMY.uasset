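; BP_HEAVY_ENEMY is an enemy NPC that attacks the first-person player character on sight.
; When PawnSensing sees the player, the enemy rotates to face them and, if able to attack, spawns a first-person projectile at SpawnProjLoc.
; Damage is applied directly to the player at firing time rather than on projectile impact.
; A Canattack flag and a short delay throttle the rate of attack.
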(event `self.PawnSensing.OnSeePawn`
  (params (Pawn :type "Pawn Object Reference"))
  (bind _asbp_first_person_character (cast `/Game/FirstPerson/Blueprints/BP_FirstPersonCharacter` Pawn))
  (`self.K2_SetActorRotation` (`KismetMathLibrary.FindRelativeLookAtRotation` (`KismetMathLibrary.Conv_VectorToTransform` (`self.K2_GetActorLocation`)) (`self.K2_GetActorLocation` _asbp_first_person_character)))
  (if (`self.canattack`)
    (`|SpawnActorFromClass` "/Game/FirstPerson/Blueprints/BP_FirstPersonProjectile.BP_FirstPersonProjectile_C" (`SceneComponent.K2_GetComponentToWorld` (`self.SpawnProjLoc`)) "Undefined" "MultiplyWithRoot" null null)
    (`GameplayStatics.ApplyDamage` _asbp_first_person_character 2.0)
    (set `self.canattack` false)
    (`KismetSystemLibrary.Delay` 1.0)
    (set `self.canattack` true)))

(fn `UserConstructionScript`)